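; Default player controller that shows the mouse cursor and provides a toggleable debug menu outside distribution builds.
; On BeginPlay, non-distribution builds create the WBP_DebugMenu widget and add the IMC_DebugInputs Enhanced Input mapping context.
; The IA_OpenDebugWindow action adds or removes the menu from the viewport, tracked by a boolean open flag.
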(event Input|EnhancedActionEvents|EnhancedInputActionIA_OpenDebugWindow
  (params (ActionValue :type Boolean) (ElapsedSeconds :type Float%20%28double-precision%29) (TriggeredSeconds :type Float%20%28double-precision%29) (InputAction :type Input%20Action%20Object%20Reference :default "/Game/Blueprints/DebugMenu/Input/IA_OpenDebugWindow.IA_OpenDebugWindow"))
  (:Started
    (if (Variables|Default|GetDebugMenuIsOpen)
      (Widget|RemovefromParent (Variables|Default|GetDebugMenu))
      (Variables|Default|SetDebugMenuIsOpen false)
      (else
        (UserInterface|Viewport|AddtoViewport (Variables|Default|GetDebugMenu) 0)
        (Variables|Default|SetDebugMenuIsOpen true)))))

(event EventBeginPlay
  (Variables|Default|SetbShowMouseCursor true)
  (if (not (Class|KismetSystemLibrary|IsPackagedforDistribution))
    (bind _returnvalue (UserInterface|CreateWidget "/Game/Blueprints/DebugMenu/WBP_DebugMenu.WBP_DebugMenu_C" self))
    (Variables|Default|SetDebugMenu _returnvalue)
    (Input|AddMappingContext (PlayerController|LocalPlayerSubsystems|GetEnhancedInputLocalPlayerSubsystem self) "/Game/Blueprints/DebugMenu/Input/IMC_DebugInputs.IMC_DebugInputs" 0 "(bIgnoreAllPressedKeysUntilRelease=True,bForceImmediately=False)")))

(fn ConstructionScript)