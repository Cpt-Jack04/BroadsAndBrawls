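; Default player pawn that acts as a camera rig, with Enhanced Input actions to zoom, pan, rotate and reset.
; Each input sets a stepped target: clamped spring arm length, actor location relative to facing, or actor yaw.
; Timelines ease from the captured start to each target, feeding their float into Interp To nodes as DeltaTime.
; Rotation ignores input while turning; reset restores only the BeginPlay zoom and position.
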(event Custom|LerpToZoomTarget
  (params (ZoomTarget :type Float%20%28double-precision%29))
  (Variables|Default|SetZoomTarget ZoomTarget)
  (Variables|Default|SetZoomStart (Variables|/Script/Engine.SpringArmComponent|GetTargetArmLength (Variables|Default|GetSpringArm)))
  (bind _lerpfloat (Timeline|ZoomLerp PlayFromStart)
    (:Update
      (bind _output_get (Variables|/Script/Engine.SpringArmComponent|SetTargetArmLength (Variables|Default|GetSpringArm) (Math|Interpolation|FInterpTo (Variables|Default|GetZoomStart) (Variables|Default|GetZoomTarget) _lerpfloat (Variables|Default|GetZoomSpeed))))
      (if (== _output_get (Variables|Default|GetZoomTarget))
        (Timeline|ZoomLerp Stop)))))

(event Custom|LerpToMoveTarget
  (params (MoveTarget :type Vector))
  (Variables|Default|SetMoveTarget MoveTarget)
  (Variables|Default|SetMoveStart (Transformation|GetActorLocation))
  (bind _lerpfloat (Timeline|MoveLerp PlayFromStart)
    (:Update
      (Transformation|SetActorLocation (Math|Interpolation|VInterpTo (Variables|Default|GetMoveStart) (Variables|Default|GetMoveTarget) _lerpfloat (Variables|Default|GetMoveSpeed)) false false)
      (if (Utilities|Operators|EqualEqual (Variables|Default|GetMoveTarget) (Transformation|GetActorLocation) 0.0)
        (Timeline|MoveLerp Stop)))))

(event Custom|LerpToRotationTarget
  (params (RotationTarget :type Rotator))
  (Variables|Default|SetRotationTarget RotationTarget)
  (Variables|Default|SetRotationStart (Transformation|GetActorRotation))
  (bind _lerpfloat (Timeline|RotateLerp PlayFromStart)
    (:Update
      (Transformation|SetActorRotation (Math|Interpolation|RInterpTo (Variables|Default|GetRotationStart) (Variables|Default|GetRotationTarget) _lerpfloat (Variables|Default|GetRotationSpeed)))
      (if (Utilities|Operators|EqualEqual (Variables|Default|GetRotationTarget) (Transformation|GetActorRotation) 0.0)
        (Variables|Default|SetIsRotating false)
        (Timeline|RotateLerp Stop)))
    (:Finished
      (Variables|Default|SetIsRotating false))))

(event Input|EnhancedActionEvents|EnhancedInputActionIA_CameraZoom
  (params (ActionValue :type Float%20%28double-precision%29) (ElapsedSeconds :type Float%20%28double-precision%29) (TriggeredSeconds :type Float%20%28double-precision%29) (InputAction :type Input%20Action%20Object%20Reference :default "/Game/Blueprints/Core/Player/Input/IA_CameraZoom.IA_CameraZoom"))
  (bind _zoomrange (Variables|Default|GetZoomRange))
  (:Triggered
    (CallFunction|LerptoZoomTarget (Math|Float|Clamp(Float) (- (Variables|/Script/Engine.SpringArmComponent|GetTargetArmLength (Variables|Default|GetSpringArm)) (* ActionValue (Variables|Default|GetZoomStep))) (.x _zoomrange) (.y _zoomrange)))))

(event Input|EnhancedActionEvents|EnhancedInputActionIA_CameraReset
  (params (ActionValue :type Boolean) (ElapsedSeconds :type Float%20%28double-precision%29) (TriggeredSeconds :type Float%20%28double-precision%29) (InputAction :type Input%20Action%20Object%20Reference :default "/Game/Blueprints/Core/Player/Input/IA_CameraReset.IA_CameraReset"))
  (:Started
    (CallFunction|LerptoZoomTarget (Variables|Default|GetZoomDefault))
    (CallFunction|LerptoMoveTarget (Variables|Default|GetPositionDefault))))

(event Input|EnhancedActionEvents|EnhancedInputActionIA_CameraMove
  (params (ActionValue :type Vector%202D%20Structure) (ElapsedSeconds :type Float%20%28double-precision%29) (TriggeredSeconds :type Float%20%28double-precision%29) (InputAction :type Input%20Action%20Object%20Reference :default "/Game/Blueprints/Core/Player/Input/IA_CameraMove.IA_CameraMove"))
  (bind _movestep (Variables|Default|GetMoveStep))
  (:Triggered
    (CallFunction|LerptoMoveTarget (+ (Variables|Default|GetMoveTarget) (* (* (.y ActionValue) _movestep) (Transformation|GetActorForwardVector)) (* (* (.x ActionValue) _movestep) (Transformation|GetActorRightVector))))))

(event Input|EnhancedActionEvents|EnhancedInputActionIA_CameraRotate
  (params (ActionValue :type Float%20%28double-precision%29) (ElapsedSeconds :type Float%20%28double-precision%29) (TriggeredSeconds :type Float%20%28double-precision%29) (InputAction :type Input%20Action%20Object%20Reference :default "/Game/Blueprints/Core/Player/Input/IA_CameraRotate.IA_CameraRotate"))
  (bind _rotationtarget (Variables|Default|GetRotationTarget))
  (:Triggered
    (if (not (Variables|Default|GetIsRotating))
      (Variables|Default|SetIsRotating true)
      (CallFunction|LerptoRotationTarget (Math|Rotator|MakeRotator (.roll _rotationtarget) (.pitch _rotationtarget) (- (.yaw _rotationtarget) (* ActionValue (Variables|Default|GetRotationStep))))))))

(event EventBeginPlay
  (Variables|Default|SetZoomDefault (Variables|/Script/Engine.SpringArmComponent|GetTargetArmLength (Variables|Default|GetSpringArm)))
  (Variables|Default|SetPositionDefault (Transformation|GetActorLocation))
  (Variables|Default|SetRotationDefault (Transformation|GetActorRotation)))

(fn ConstructionScript)